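; Server-authoritative battle royale safe zone that shrinks in phases and registers itself with BRGameState.
; Once enabled, a timer alternates holds with shrinks that rescale the wall and interpolate it toward a random next center.
; Each phase multiplies radius and timings until the minimum radius is passed.
; While enabled, every tick damages living players outside the horizontal radius, skipping those in the plane, without delta-time scaling.
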(event `self.ReceiveTick`
  (params (DeltaSeconds :type "Float (single-precision)"))
  (if (`self.EstasEncongiendote?`)
    (`self.ActualizaLaPared` DeltaSeconds))
  (if (`self.EstaHabilitadoElSafeZone?`)
    (`/Engine/EditorBlueprintResources/ActorMacros.Switch Has Authority`
      (:`Authority`
        (`self.DañaJugadoresAfueraDeLaPared` DeltaSeconds)))))

(event `ComienzaAEncoger`
  (`/Engine/EditorBlueprintResources/ActorMacros.Switch Has Authority`
    (:`Authority`
      (`/Engine/EditorBlueprintResources/StandardMacros.IncrementInt` (`self.NumeroVecesParaEncoger`)
        (:`  `
          (set `self.PosicionDeInicio` (`self.K2_GetActorLocation`))
          (set `self.EstasEncongiendote?` true)
          (set `self.ComienzaTiempoDeEncogimiento` (`GameplayStatics.GetTimeSeconds`))
          (set `self.VelocidadDeEncogimiento` (/ (- (`self.Radio`) (`self.SiguienteRadio`)) (`self.TiempoDeEncogimiento`)))
          (`self.SetActorHiddenInGame` false))))))

(event `HabiltaElSafeZone`
  (`/Engine/EditorBlueprintResources/ActorMacros.Switch Has Authority`
    (:`Authority`
      (set `self.EstaHabilitadoElSafeZone?` true)
      (`KismetSystemLibrary.K2_SetTimerDelegate` (delegate `ComienzaAEncoger`) (`self.RetencionDeTiempo`)))))

(event `self.ReceiveBeginPlay`
  (`/Engine/EditorBlueprintResources/ActorMacros.Switch Has Authority`
    (:`Authority`
      (bind _asbrgame_state (cast `/Game/FirstPersonBP/Blueprints/BRGameState` (`GameplayStatics.GetGameState`)))
      (set `/Game/FirstPersonBP/Blueprints/BRGameState.SafeZone` self _asbrgame_state)
      (set `self.SiguienteRadio` (* (`self.Radio`) (`self.MultiplicadorDeEncongimiento`)))
      (set `self.VelocidadDeEncogimiento` (/ (- (`self.Radio`) (`self.SiguienteRadio`)) (`self.TiempoDeEncogimiento`)))
      (set `self.SiguientePosicion` (`self.GetSiguientePosicion`)))))

(event `ActualizaLaPared`
  (params (TiempoDelta :type "Float (double-precision)"))
  (bind _radio (`self.Radio`))
  (`/Engine/EditorBlueprintResources/ActorMacros.Switch Has Authority`
    (:`Authority`
      (set `self.Radio` (- (`self.Radio`) (* (`self.VelocidadDeEncogimiento`) TiempoDelta)))
      (`self.SetActorScale3D` (`KismetMathLibrary.MakeVector` _radio _radio (`self.Altura`)))
      (`self.K2_SetActorLocation` (`KismetMathLibrary.VInterpTo` (`self.K2_GetActorLocation`) (`self.SiguientePosicion`) TiempoDelta (/ (`KismetMathLibrary.VSize` (- (`self.PosicionDeInicio`) (`self.SiguientePosicion`))) (`self.TiempoDeEncogimiento`))))
      (if (and (`self.HasAuthority`) (>= (/ (- (`GameplayStatics.GetTimeSeconds`) (`self.ComienzaTiempoDeEncogimiento`)) (`self.TiempoDeEncogimiento`)) 1.0))
        (set `self.EstasEncongiendote?` false)
        (set `self.RetencionDeTiempo` (* (`self.RetencionDeTiempo`) (`self.MultiplicadorDeTiempo`)))
        (set `self.SiguienteRadio` (* (`self.SiguienteRadio`) (`self.MultiplicadorDeEncongimiento`)))
        (set `self.SiguientePosicion` (`self.GetSiguientePosicion`))
        (set `self.TiempoDeEncogimiento` (* (`self.TiempoDeEncogimiento`) (`self.MultiplicadorDeTiempo`)))
        (if (>= (`self.Radio`) (`self.RadioMinimo`))
          (`KismetSystemLibrary.K2_SetTimerDelegate` (delegate `ComienzaAEncoger`) (`self.RetencionDeTiempo`))
          (else
            (set `self.FinalizadoEncogimiento?` true)))))))

(event `DañaJugadoresAfueraDeLaPared`
  (params (TiempoDelta :type "Float (double-precision)"))
  (if (and (>= (`self.NumeroVecesParaEncoger`) 0) (`self.EstaHabilitadoElSafeZone?`))
    (bind _asbrgame_mode (cast `/Game/FirstPersonBP/Blueprints/BRGameMode` (`GameplayStatics.GetGameMode`)))
    (for _array_element (`/Game/FirstPersonBP/Blueprints/BRGameMode.ListaDeJugadoresVivos` _asbrgame_mode)
      (bind _returnvalue (`Controller.K2_GetPawn` _array_element))
      (if (and (not (`/Game/FirstPersonBP/Blueprints/BPPlayerController.EstasEnElAvion` _array_element)) (> (`self.GetHorizontalDistanceTo` _returnvalue) (/ (`self.Radio`) 2.0)))
        (`KismetSystemLibrary.PrintString` "Me pega la tormenta")
        (`GameplayStatics.ApplyDamage` _returnvalue (`self.DañoPorPared`) (`Pawn.GetController` _returnvalue) self "/Script/Engine.DamageType")))))

(fn `GetSiguientePosicion`
  (returns (SiguientePosicion :type "Vector Structure"))
  (bind _returnvalue (`self.K2_GetActorLocation`))
  (bind _z (.z _returnvalue))
  (bind _returnvalue_2 (* (- (`self.Radio`) (`self.SiguienteRadio`)) 0.5))
  (bind _returnvalue_3 (* _returnvalue_2 -1.0))
  (return (`KismetMathLibrary.MakeVector` (.x (+ _returnvalue (`KismetMathLibrary.MakeVector` (* (`KismetMathLibrary.DegCos` (`KismetMathLibrary.RandomFloatInRange` -180.0 180.0)) (`KismetMathLibrary.RandomFloatInRange` _returnvalue_3 _returnvalue_2)) (* (`KismetMathLibrary.DegSin` (`KismetMathLibrary.RandomFloatInRange` -180.0 180.0)) (`KismetMathLibrary.RandomFloatInRange` _returnvalue_3 _returnvalue_2)) _z))) (.y (+ _returnvalue (`KismetMathLibrary.MakeVector` (* (`KismetMathLibrary.DegCos` (`KismetMathLibrary.RandomFloatInRange` -180.0 180.0)) (`KismetMathLibrary.RandomFloatInRange` _returnvalue_3 _returnvalue_2)) (* (`KismetMathLibrary.DegSin` (`KismetMathLibrary.RandomFloatInRange` -180.0 180.0)) (`KismetMathLibrary.RandomFloatInRange` _returnvalue_3 _returnvalue_2)) _z))) _z)))

(fn `UserConstructionScript`
  (bind _radio (`self.Radio`))
  (`SceneComponent.SetWorldScale3D` (`self.SafeZone`) (`KismetMathLibrary.MakeVector` _radio _radio (`self.Altura`))))