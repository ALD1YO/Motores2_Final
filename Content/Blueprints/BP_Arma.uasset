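; Weapon Blueprint that manages magazine and reserve ammo for its owning FirstPersonCharacter.
; On authority, BeginPlay fills the magazine, sets starting reserve and caches the owner, while Disparando decrements rounds and triggers Recarga when empty.
; Recarga flags the player as reloading during a fixed delay, then refills from reserve.
; AgregarBalas, also authority-only, tops up the magazine and sends surplus to the capped reserve.
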(event `Recarga`
  (bind _returnvalue (`KismetMathLibrary.Min` (`self.CantidadDeBalasDeRepuesto`) (`self.TamañoDelCargadorDelArma`)))
  ;[1 1 1] Recarga
  (set `/Game/FirstPersonBP/Blueprints/FirstPersonCharacter.EstasRecargando?` true (`self.Jugador`))
  (`KismetSystemLibrary.Delay` 2.0)
  (set `self.CantidadDeBalasEnElArma` _returnvalue)
  (set `self.CantidadDeBalasDeRepuesto` (`KismetMathLibrary.Max` (- (`self.CantidadDeBalasDeRepuesto`) _returnvalue)))
  (set `/Game/FirstPersonBP/Blueprints/FirstPersonCharacter.EstasRecargando?` false (`self.Jugador`)))

(event `Disparando`
  (bind _cantidaddebalasenelarma (`self.CantidadDeBalasEnElArma`))
  ;[1 1 1] Dispara Jugador
  (`/Engine/EditorBlueprintResources/ActorMacros.Switch Has Authority`
    (:`Authority`
      (`/Engine/EditorBlueprintResources/StandardMacros.DecrementInt` _cantidaddebalasenelarma
        (:`  `
          (if (<= _cantidaddebalasenelarma 0)
            (`self.Recarga`)))))))

(event `AgregarBalas`
  (params (CantidadDeBalas :type Integer))
  (bind _returnvalue (`KismetMathLibrary.Min` CantidadDeBalas (- (`self.TamañoDelCargadorDelArma`) (`self.CantidadDeBalasEnElArma`))))
  (bind _returnvalue_2 (- CantidadDeBalas _returnvalue))
  ;[1 1 1] Dar Balas
  (`/Engine/EditorBlueprintResources/ActorMacros.Switch Has Authority`
    (:`Authority`
      (set `self.CantidadDeBalasEnElArma` (+ (`self.CantidadDeBalasEnElArma`) _returnvalue))
      (if (> _returnvalue_2 0)
        (set `self.CantidadDeBalasDeRepuesto` (+ (`self.CantidadDeBalasDeRepuesto`) (`KismetMathLibrary.Min` _returnvalue_2 (- (`self.CantidadDeBalasMaximaDeRepuesto`) (`self.CantidadDeBalasDeRepuesto`)))))))))

(event `self.ReceiveBeginPlay`
  ;[1 1 1] Empieza el juego
  (`/Engine/EditorBlueprintResources/ActorMacros.Switch Has Authority`
    (:`Authority`
      (set `self.CantidadDeBalasEnElArma` (`self.TamañoDelCargadorDelArma`))
      (set `self.CantidadDeBalasDeRepuesto` (`self.CantidadDeBalasConLasQueEmpieza`))
      (bind _asfirst_person_character (cast `/Game/FirstPersonBP/Blueprints/FirstPersonCharacter` (`self.GetOwner`)))
      (set `self.Jugador` _asfirst_person_character))))

(fn `UserConstructionScript`)