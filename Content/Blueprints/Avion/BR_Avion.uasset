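; Battle royale plane actor that flies a random straight route across the map at a fixed altitude.
; On BeginPlay the authority picks an edge start point and a roughly opposite end point with slight angular jitter, orients the plane and configures its spring arm.
; Tick moves it toward the end at constant speed.
; Its lifespan is map size divided by speed.
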(event `self.ReceiveBeginPlay`
  (bind _springarm (`self.SpringArm`))
  (`/Engine/EditorBlueprintResources/ActorMacros.Switch Has Authority`
    (:`Authority`
      (set `SpringArmComponent.TargetArmLength` 200.0 _springarm)
      (set `SpringArmComponent.TargetOffset` (0.0 0.0 100.0) _springarm)
      (`self.SetLifeSpan` (/ (`self.TamañoDelMapa`) (`self.Velocidad`)))
      (bind _output_get (set `self.OffsetDeCentro` (`KismetMathLibrary.Normal` (`KismetMathLibrary.MakeVector` (`KismetMathLibrary.DegCos` (`KismetMathLibrary.RandomFloatInRange` -180.0 180.0)) (`KismetMathLibrary.DegSin` (`KismetMathLibrary.RandomFloatInRange` -180.0 180.0))))))
      (set `self.PuntoDeInicioDeVuelo` (* _output_get (/ (`self.TamañoDelMapa`) 2.0)))
      (set `self.PuntoFinalDeVuelo` (* (`KismetMathLibrary.GreaterGreater_VectorRotator` (* (`self.OffsetDeCentro`) -1.0) (`KismetMathLibrary.MakeRotator` 0.0 0.0 (`KismetMathLibrary.RandomFloatInRange` -15.0 15.0))) (/ (`self.TamañoDelMapa`) 2.0)))
      (`self.K2_SetActorRotation` (`KismetMathLibrary.MakeRotator` (.roll (`KismetMathLibrary.MakeRotFromX` (- (`self.PuntoFinalDeVuelo`) (`self.PuntoDeInicioDeVuelo`)))) (.pitch (`KismetMathLibrary.MakeRotFromX` (- (`self.PuntoFinalDeVuelo`) (`self.PuntoDeInicioDeVuelo`)))) (+ (.yaw (`KismetMathLibrary.MakeRotFromX` (- (`self.PuntoFinalDeVuelo`) (`self.PuntoDeInicioDeVuelo`)))) 90.0)))
      (`self.K2_SetActorLocation` (`self.PuntoDeInicioDeVuelo`)))))

(event `self.ReceiveTick`
  (params (DeltaSeconds :type "Float (single-precision)"))
  (`self.K2_SetActorLocation` (`KismetMathLibrary.MakeVector` (.x (`KismetMathLibrary.VInterpTo_Constant` (`self.K2_GetActorLocation`) (`self.PuntoFinalDeVuelo`) DeltaSeconds (`self.Velocidad`))) (.y (`KismetMathLibrary.VInterpTo_Constant` (`self.K2_GetActorLocation`) (`self.PuntoFinalDeVuelo`) DeltaSeconds (`self.Velocidad`))) (`self.Altitud`))))

(fn `UserConstructionScript`)