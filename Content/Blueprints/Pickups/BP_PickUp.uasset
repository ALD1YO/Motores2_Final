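; BP_PickUp is a pickup actor with a spinning mesh and a sphere that detects the first-person character.
; Tick yaws PickUpMesh at a steady rate, then zeroes its world pitch and roll to keep it upright.
; Sphere overlaps cast to FirstPersonCharacter and call player-entering and player-leaving events, left empty here as apparent hooks for child pickups.
; A hit on the sphere switches off its physics simulation.
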(event `self.ReceiveTick`
  (params (DeltaSeconds :type "Float (single-precision)"))
  ;[1 1 1] Construye y ajusta la rotación del mesh
  (`SceneComponent.K2_AddRelativeRotation` (`self.PickUpMesh`) (`KismetMathLibrary.MakeRotator` 0.0 0.0 (* DeltaSeconds 180.0)) false false)
  (`SceneComponent.K2_SetWorldRotation` (`self.PickUpMesh`) (`KismetMathLibrary.MakeRotator` 0.0 0.0 (.yaw (`SceneComponent.K2_GetComponentRotation` (`self.PickUpMesh`)))) false false))

(event `PickUp_JugadorEntrando`
  (params (Jugador :type "/Game/FirstPersonBP/Blueprints/FirstPersonCharacter Object Reference")))

(event `PickUp_JugadorSaliendo`
  (params (Jugador :type "/Game/FirstPersonBP/Blueprints/FirstPersonCharacter Object Reference")))

(event `self.PickUpSphere.OnComponentEndOverlap`
  (params (OverlappedComponent :type "PrimitiveComponent Object Reference") (OtherActor :type "Actor Object Reference") (OtherComp :type "PrimitiveComponent Object Reference") (OtherBodyIndex :type Integer))
  (bind _asfirst_person_character (cast `/Game/FirstPersonBP/Blueprints/FirstPersonCharacter` OtherActor))
  (`self.PickUp_JugadorSaliendo` _asfirst_person_character))

(event `self.PickUpSphere.OnComponentBeginOverlap`
  (params (OverlappedComponent :type "PrimitiveComponent Object Reference") (OtherActor :type "Actor Object Reference") (OtherComp :type "PrimitiveComponent Object Reference") (OtherBodyIndex :type Integer) (bFromSweep :type Boolean) (SweepResult :type "HitResult Structure (by ref)"))
  (bind _asfirst_person_character (cast `/Game/FirstPersonBP/Blueprints/FirstPersonCharacter` OtherActor))
  (`self.PickUp_JugadorEntrando` _asfirst_person_character))

(event `self.PickUpSphere.OnComponentHit`
  (params (HitComponent :type "PrimitiveComponent Object Reference") (OtherActor :type "Actor Object Reference") (OtherComp :type "PrimitiveComponent Object Reference") (NormalImpulse :type "Vector Structure") (Hit :type "HitResult Structure (by ref)"))
  (`PrimitiveComponent.SetSimulatePhysics` (`self.PickUpSphere`) false))

(fn `UserConstructionScript`)