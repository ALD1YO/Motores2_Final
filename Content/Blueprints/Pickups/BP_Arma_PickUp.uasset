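; BP_Arma_PickUp is a weapon pickup that represents the weapon class set in ArmaAsignar and carries its ammo counts.
; On BeginPlay, only the authority copies magazine and reserve bullet counts from that class's defaults.
; When a player enters, it registers itself as that player's ArmaPickUp.
; On exit, it clears that reference only if it still points to this pickup.
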(event `self.ReceiveBeginPlay`
  (bind (_damage _nombre _cantidaddebalasderepuesto _cantidaddebalasconlasqueempieza _cantidaddebalasenelarma) (defaults `/Game/Blueprints/Pickups/BP_Arma_PickUp` (`self.ArmaAsignar`)))
  ;[1 1 1] Asigna Balas al inicio del juego
  (`/Engine/EditorBlueprintResources/ActorMacros.Switch Has Authority`
    (:`Authority`
      (set `self.BalasQueTieneCargador` _cantidaddebalasenelarma)
      (set `self.BalasDeRespuesto` _cantidaddebalasderepuesto))))

(event `self.PickUp_JugadorEntrando`
  (params (Jugador :type "/Game/FirstPersonBP/Blueprints/FirstPersonCharacter Object Reference"))
  (set `/Game/FirstPersonBP/Blueprints/FirstPersonCharacter.ArmaPickUp` self Jugador))

(event `self.PickUp_JugadorSaliendo`
  (params (Jugador :type "/Game/FirstPersonBP/Blueprints/FirstPersonCharacter Object Reference"))
  (if (== (`/Game/FirstPersonBP/Blueprints/FirstPersonCharacter.ArmaPickUp` Jugador) self)
    (set `/Game/FirstPersonBP/Blueprints/FirstPersonCharacter.ArmaPickUp` null Jugador)))

(fn `UserConstructionScript`
  (`parent.UserConstructionScript`))