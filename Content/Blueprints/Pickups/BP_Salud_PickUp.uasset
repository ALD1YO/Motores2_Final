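; Health pickup Blueprint that heals the player who enters it and then destroys itself.
; On the PickUpJugadorEntrando event, only the authority calls ModificarSalud on the player with the negated CantidadDeSalud.
; The pickup is consumed when the player's health is below or exactly at SaludMaxima, so it is used up even at full health.
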(event `self.PickUp_JugadorEntrando`
  (params (Jugador :type "/Game/FirstPersonBP/Blueprints/FirstPersonCharacter Object Reference"))
  (bind _saluddelpersonaje (`/Game/FirstPersonBP/Blueprints/FirstPersonCharacter.SaludDelPersonaje` Jugador))
  (bind _saludmaxima (`/Game/FirstPersonBP/Blueprints/FirstPersonCharacter.SaludMaxima` Jugador))
  (`/Engine/EditorBlueprintResources/ActorMacros.Switch Has Authority`
    (:`Authority`
      (if (< _saluddelpersonaje _saludmaxima)
        (`/Game/FirstPersonBP/Blueprints/FirstPersonCharacter.ModificarSalud` Jugador (* (`self.CantidadDeSalud`) -1) :!label _label)
        (`self.K2_DestroyActor`)
        (elif (== _saluddelpersonaje _saludmaxima)
          (goto _label))))))

(fn `UserConstructionScript`
  (`parent.UserConstructionScript`))